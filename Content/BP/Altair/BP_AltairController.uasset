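; BP_AltairController is a controller that passes player movement input to the BP_Altair pawn.
; On BeginPlay it casts player pawn 0 to BP_Altair and stores the reference.
; MoveForward and MoveRight axes call Altair's Move with a forward flag, and the Sprint action starts and stops sprinting on press and release.
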(event EventBeginPlay
  (bind _asbp_altair (Utilities|Casting|CastToBP_Altair (Game|Player|GetPlayerPawn 0)))
  (Variables|Default|SetAltair _asbp_altair))

(event EventTick
  (params (DeltaSeconds :type Float%20%28single-precision%29)))

(event Input|ActionEvents|InputActionSprint
  (params (Key :type Key%20Structure :default "None"))
  (bind _altair (Variables|Default|GetAltair))
  (:Pressed
    (Default|StartSprinting _altair))
  (:Released
    (Default|StopSprinting _altair)))

(event Input|AxisEvents|InputAxisMoveForward
  (params (AxisValue :type Float%20%28single-precision%29))
  (Default|Move (Variables|Default|GetAltair) AxisValue true))

(event Input|AxisEvents|InputAxisMoveRight
  (params (AxisValue :type Float%20%28single-precision%29))
  (Default|Move (Variables|Default|GetAltair) AxisValue false))

(fn ConstructionScript)