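; BP_Altair is a character Blueprint that provides camera-relative planar movement and sprinting.
; Its Move event uses only the control rotation's yaw to pick a forward or right vector for movement input, keeping motion on the ground plane.
; BeginPlay caches the default max walk speed, which sprint events swap with SprintSpeed and restore through small helper functions.
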(event Custom|Move
  (params (AxisValue :type Float%20%28single-precision%29) (Forward? :type Boolean))
  (bind _returnvalue (Pawn|GetControlRotation :!class /Script/Engine.Pawn))
  (bind _yaw (Math|Rotator|BreakRotator _returnvalue))
  (bind _returnvalue_2 (Math|Rotator|MakeRotator 0.0 0.0 _yaw))
  (Pawn|Input|AddMovementInput (Math|Vector|SelectVector (Math|Vector|GetForwardVector _returnvalue_2) (Math|Vector|GetRightVector _returnvalue_2) Forward?) AxisValue false))

(event Custom|StartSprinting
  (CallFunction|ModifyWalkingSpeed (Variables|Default|GetSprintSpeed)))

(event Custom|StopSprinting
  (CallFunction|ResetWalkingSpeed))

(event EventBeginPlay
  (Variables|Default|SetWalkSpeed (Variables|/Script/Engine.CharacterMovementComponent|GetMaxWalkSpeed (Variables|Character|GetCharacterMovement))))

(event Collision|EventActorBeginOverlap
  (params (OtherActor :type Actor%20Object%20Reference)))

(event EventTick
  (params (DeltaSeconds :type Float%20%28single-precision%29)))

(fn ConstructionScript)

(fn ModifyWalkingSpeed
  (params (NewSpeed :type Float%20%28single-precision%29))
  (Variables|/Script/Engine.CharacterMovementComponent|SetMaxWalkSpeed (Variables|Character|GetCharacterMovement) NewSpeed))

(fn ResetWalkingSpeed
  (Variables|/Script/Engine.CharacterMovementComponent|SetMaxWalkSpeed (Variables|Character|GetCharacterMovement) (Variables|Default|GetWalkSpeed)))